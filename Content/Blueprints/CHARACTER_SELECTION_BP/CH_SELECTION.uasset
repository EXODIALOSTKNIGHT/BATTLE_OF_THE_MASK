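; CH_SELECTION is a character selection Blueprint that swaps a player's current pawn for a chosen character class.
; When CHANGESTATUS is false, its SWAP event destroys any valid controlled pawn, spawns the chosen class and has the given controller possess it.
; The spawn transform comes from the SPAWN actor array through a random index whose Min and Max inputs are reversed.
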(event Custom|SWAP
  (params (PLAYER%20CONTROLLER :type Player%20Controller%20Object%20Reference) (CHARACTER :type Character%20Class%20Reference) (CHANGE%20STATUS :type Boolean))
  (bind _returnvalue (Pawn|GetControlledPawn PLAYER%20CONTROLLER))
  (bind _spawn (Variables|Default|GetSPAWN))
  ;[1 1 1] SWAP CURRENT CHARACTER WITH SELECTED CHARACTER
  (if (not CHANGE%20STATUS)
    (Utilities|IsValid _returnvalue
      (:Is%20Valid
        (Actor|DestroyActor _returnvalue))
      (:Is%20Not%20Valid
        _))
    (bind _returnvalue_2 (Game|SpawnActorfromClass CHARACTER (Transformation|GetActorTransform (Utilities|Array|Get(acopy) _spawn (Math|Random|RandomIntegerinRange (- (Utilities|Array|Length _spawn) 1) 0))) "Undefined" 0 0))
    (Pawn|Possess PLAYER%20CONTROLLER _returnvalue_2)))

(fn ConstructionScript)