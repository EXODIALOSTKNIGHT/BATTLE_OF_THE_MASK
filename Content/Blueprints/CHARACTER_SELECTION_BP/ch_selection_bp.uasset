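; Character selection Blueprint that moves a highlight across four mask meshes with the Left and Right keys.
; Tick polls the keys through 0.2-second Delays, steps a clamped LeftRight index, then applies the selection material to that mask and Lambert materials to the others.
; An unfinished confirm branch, marked as Enter, also checks Left and opens Arena1 for every index, without passing on the chosen character.
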(event EventTick
  (params (DeltaSeconds :type Float%20%28single-precision%29))
  ;[1 1 1] CHARACTER SELECTION control
  (Utilities|FlowControl|Sequence
    (:then_0
      (Utilities|FlowControl|Delay 0.2)
      (if (Game|Player|IsInputKeyDown (Game|GetPlayerController 0) "Right")
        (if (< (Variables|Default|Getleft_right) 3)
          (bind _output_get (Variables|Default|Setleft_right (+ (Variables|Default|Getleft_right) 1)))
          (switch int _output_get
            (:0
              (Rendering|Material|SetMaterial (Variables|Default|GetMASK_1) 0 "/Game/MATERIALS/SELECTION_MATERIALS.SELECTION_MATERIALS")
              (Rendering|Material|SetMaterial (Variables|Default|GetMASK_2) 0 "/Game/CHARACTERS/MASK_2/MATERIALS/lambert2.lambert2")
              (Rendering|Material|SetMaterial (Variables|Default|GetMASK_3) 0 "/Game/CHARACTERS/MASK_3/MATERIALS/lambert3.lambert3")
              (Rendering|Material|SetMaterial (Variables|Default|GetMASK_4) 0 "/Game/CHARACTERS/MASK_4/MATERIALS/lambert4.lambert4"))
            (:1
              (Rendering|Material|SetMaterial (Variables|Default|GetMASK_2) 0 "/Game/MATERIALS/SELECTION_MATERIALS.SELECTION_MATERIALS")
              (Rendering|Material|SetMaterial (Variables|Default|GetMASK_1) 0 "/Game/CHARACTERS/MASK_1/MATERIALS/lambert1.lambert1")
              (Rendering|Material|SetMaterial (Variables|Default|GetMASK_3) 0 "/Game/CHARACTERS/MASK_3/MATERIALS/lambert3.lambert3")
              (Rendering|Material|SetMaterial (Variables|Default|GetMASK_4) 0 "/Game/CHARACTERS/MASK_4/MATERIALS/lambert4.lambert4"))
            (:2
              (Rendering|Material|SetMaterial (Variables|Default|GetMASK_3) 0 "/Game/MATERIALS/SELECTION_MATERIALS.SELECTION_MATERIALS")
              (Rendering|Material|SetMaterial (Variables|Default|GetMASK_1) 0 "/Game/CHARACTERS/MASK_1/MATERIALS/lambert1.lambert1")
              (Rendering|Material|SetMaterial (Variables|Default|GetMASK_2) 0 "/Game/CHARACTERS/MASK_2/MATERIALS/lambert2.lambert2")
              (Rendering|Material|SetMaterial (Variables|Default|GetMASK_4) 0 "/Game/CHARACTERS/MASK_4/MATERIALS/lambert4.lambert4"))
            (:3
              (Rendering|Material|SetMaterial (Variables|Default|GetMASK_4) 0 "/Game/MATERIALS/SELECTION_MATERIALS.SELECTION_MATERIALS")
              (Rendering|Material|SetMaterial (Variables|Default|GetMASK_1) 0 "/Game/CHARACTERS/MASK_1/MATERIALS/lambert1.lambert1")
              (Rendering|Material|SetMaterial (Variables|Default|GetMASK_2) 0 "/Game/CHARACTERS/MASK_2/MATERIALS/lambert2.lambert2")
              (Rendering|Material|SetMaterial (Variables|Default|GetMASK_3) 0 "/Game/CHARACTERS/MASK_3/MATERIALS/lambert3.lambert3"))))))
    (:then_1
      (Utilities|FlowControl|Delay 0.2)
      (if (Game|Player|IsInputKeyDown (Game|GetPlayerController 0) "Left")
        (if (> (Variables|Default|Getleft_right) 0)
          (bind _output_get_2 (Variables|Default|Setleft_right (- (Variables|Default|Getleft_right) 1)))
          (switch int _output_get_2
            (:0
              (Rendering|Material|SetMaterial (Variables|Default|GetMASK_1) 0 "/Game/MATERIALS/SELECTION_MATERIALS.SELECTION_MATERIALS")
              (Rendering|Material|SetMaterial (Variables|Default|GetMASK_2) 0 "/Game/CHARACTERS/MASK_2/MATERIALS/lambert2.lambert2")
              (Rendering|Material|SetMaterial (Variables|Default|GetMASK_3) 0 "/Game/CHARACTERS/MASK_3/MATERIALS/lambert3.lambert3")
              (Rendering|Material|SetMaterial (Variables|Default|GetMASK_4) 0 "/Game/CHARACTERS/MASK_4/MATERIALS/lambert4.lambert4"))
            (:1
              (Rendering|Material|SetMaterial (Variables|Default|GetMASK_2) 0 "/Game/MATERIALS/SELECTION_MATERIALS.SELECTION_MATERIALS")
              (Rendering|Material|SetMaterial (Variables|Default|GetMASK_1) 0 "/Game/CHARACTERS/MASK_1/MATERIALS/lambert1.lambert1")
              (Rendering|Material|SetMaterial (Variables|Default|GetMASK_3) 0 "/Game/CHARACTERS/MASK_3/MATERIALS/lambert3.lambert3")
              (Rendering|Material|SetMaterial (Variables|Default|GetMASK_4) 0 "/Game/CHARACTERS/MASK_4/MATERIALS/lambert4.lambert4"))
            (:2
              (Rendering|Material|SetMaterial (Variables|Default|GetMASK_3) 0 "/Game/MATERIALS/SELECTION_MATERIALS.SELECTION_MATERIALS")
              (Rendering|Material|SetMaterial (Variables|Default|GetMASK_1) 0 "/Game/CHARACTERS/MASK_1/MATERIALS/lambert1.lambert1")
              (Rendering|Material|SetMaterial (Variables|Default|GetMASK_2) 0 "/Game/CHARACTERS/MASK_2/MATERIALS/lambert2.lambert2")
              (Rendering|Material|SetMaterial (Variables|Default|GetMASK_4) 0 "/Game/CHARACTERS/MASK_4/MATERIALS/lambert4.lambert4"))
            (:3
              (Rendering|Material|SetMaterial (Variables|Default|GetMASK_4) 0 "/Game/MATERIALS/SELECTION_MATERIALS.SELECTION_MATERIALS")
              (Rendering|Material|SetMaterial (Variables|Default|GetMASK_1) 0 "/Game/CHARACTERS/MASK_1/MATERIALS/lambert1.lambert1")
              (Rendering|Material|SetMaterial (Variables|Default|GetMASK_2) 0 "/Game/CHARACTERS/MASK_2/MATERIALS/lambert2.lambert2")
              (Rendering|Material|SetMaterial (Variables|Default|GetMASK_3) 0 "/Game/CHARACTERS/MASK_3/MATERIALS/lambert3.lambert3"))))))
    (:then_2
      ;[1 1 1] ENTER NOT FINISH
      (Utilities|FlowControl|Delay 0.2)
      (if (Game|Player|IsInputKeyDown (Game|GetPlayerController 0) "Left")
        (switch int (Variables|Default|Getleft_right)
          (:0
            (Game|OpenLevel(byName) "Arena1"))
          (:1
            (Game|OpenLevel(byName) "Arena1"))
          (:2
            (Game|OpenLevel(byName) "Arena1"))
          (:3
            (Game|OpenLevel(byName) "Arena1")))))))

(fn ConstructionScript)