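; BOTM is a Blueprint that handles respawning player pawns, caching PlayerStart0 actors as spawn points on BeginPlay.
; SpawnCharacter destroys a controller's existing pawn, spawns and possesses a MASK_1_BP, and sets the view to GameCamera.
; DespawnPlayer mirrors this flow, but its spawn class and possess target are empty.
; GetRandomSpawn holds an unconnected random spawn-point lookup with reversed Min/Max inputs.
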(event Custom|Spawn%20Character
  (params (PlayerController :type Player%20Controller%20Object%20Reference))
  (bind _returnvalue (Pawn|GetControlledPawn PlayerController))
  (Utilities|IsValid _returnvalue
    (:Is%20Valid
      (Actor|DestroyActor _returnvalue)
      (bind _returnvalue_2 (Game|SpawnActorfromClass "/Game/CHARACTERS/MASK_1/BLUEPRINT/MASK_1_BP.MASK_1_BP_C" (Utilities|GetRandomSpawn) "Undefined" 0 0))
      (Pawn|Possess PlayerController _returnvalue_2)
      (Game|Player|SetViewTargetwithBlend PlayerController (Variables|Default|GetGameCamera) 0.0 "VTBlend_Linear" 0.0 false))))

(event Custom|Despawn%20Player
  (params (PlayerController :type Player%20Controller%20Object%20Reference))
  (bind _returnvalue (Pawn|GetControlledPawn PlayerController))
  (Utilities|IsValid _returnvalue
    (:Is%20Valid
      (Actor|DestroyActor _returnvalue)
      (Game|SpawnActorfromClass 0 (Utilities|GetRandomSpawn) "Undefined" 0 0)
      (Pawn|Possess PlayerController)
      (Game|Player|SetViewTargetwithBlend PlayerController (Variables|Default|GetGameCamera) 0.0 "VTBlend_Linear" 0.0 false))))

(event EventBeginPlay
  (bind _outactors (Actor|GetAllActorsOfClass "/Game/CHARACTERS/MASK_1/PlayerStart0.PlayerStart0_C"))
  (Variables|Default|SetSpawnPoint _outactors))

(fn ConstructionScript)