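; CONTROLLER_CH_BP is an input controller Blueprint that moves player 0's character along fixed world axes.
; Four axis events (FORWARD, BACKWARD, LEFT, RIGHT) each call AddMovementInput with a signed X or Y direction, independent of character or camera rotation.
; Each axis value feeds both the direction vector and the scale, so input response is squared and the hardcoded sign determines direction.
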(event Input|AxisEvents|InputAxisFORWARD
  (params (AxisValue :type Float%20%28single-precision%29))
  (Pawn|Input|AddMovementInput (Game|GetPlayerCharacter 0) (Math|Vector|MakeVector (* (Input|AxisValues|GetFORWARD) 1.0) 0.0 0.0) AxisValue false))

(event Input|AxisEvents|InputAxisBACKWARD
  (params (AxisValue :type Float%20%28single-precision%29))
  (Pawn|Input|AddMovementInput (Game|GetPlayerCharacter 0) (Math|Vector|MakeVector (* (Input|AxisValues|GetBACKWARD) -1.0) 0.0 0.0) AxisValue false))

(event Input|AxisEvents|InputAxisRIGHT
  (params (AxisValue :type Float%20%28single-precision%29))
  (Pawn|Input|AddMovementInput (Game|GetPlayerCharacter 0) (Math|Vector|MakeVector 0.0 (* (Input|AxisValues|GetRIGHT) 1.0) 0.0) AxisValue false))

(event Input|AxisEvents|InputAxisLEFT
  (params (AxisValue :type Float%20%28single-precision%29))
  (Pawn|Input|AddMovementInput (Game|GetPlayerCharacter 0) (Math|Vector|MakeVector 0.0 (* (Input|AxisValues|GetLEFT) -1.0) 0.0) AxisValue false))

(fn ConstructionScript)