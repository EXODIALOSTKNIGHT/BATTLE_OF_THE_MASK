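; Shared camera actor that keeps four player characters in frame by following their average position and zooming with their spread.
; Each tick it finds the center and the largest pairwise distance between players 0–3, with no check for missing ones.
; A Box moved to that center drives the spring arm's smoothed, offset XY position at fixed starting height.
; Arm length interpolates toward that distance, reduced by a margin and clamped.
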(event Custom|CameraZoom
  (bind _springarm (Variables|Default|GetSpringArm))
  ;[1 1 1] Camera Zoom
  (Variables|/Script/Engine.SpringArmComponent|SetTargetArmLength _springarm (Math|Interpolation|FInterpTo (Variables|/Script/Engine.SpringArmComponent|GetTargetArmLength _springarm) (Math|Float|Max(Float) (Math|Float|Min(Float) (Variables|Default|GetLongestDistance) 2e+03) 0.0) (Variables|Default|GetDelta) 3.0)))

(event Custom|SetLongestPoint
  (bind _returnvalue (Game|GetPlayerCharacter 0))
  (bind _returnvalue_2 (Game|GetPlayerCharacter 1))
  (bind _returnvalue_3 (Game|GetPlayerCharacter 2))
  (bind _returnvalue_4 (Game|GetPlayerCharacter 3))
  ;[1 1 1] check longest distance between 2 players
  (Variables|Default|SetLongestDistance (- (.MaxValue (Math|Float|MaxOfFloatArray (Utilities|Array|MakeArray (Transformation|GetDistanceTo _returnvalue _returnvalue_2) (Transformation|GetDistanceTo _returnvalue _returnvalue_3) (Transformation|GetDistanceTo _returnvalue _returnvalue_4) (Transformation|GetDistanceTo _returnvalue_2 _returnvalue_3) (Transformation|GetDistanceTo _returnvalue_2 _returnvalue_4) (Transformation|GetDistanceTo _returnvalue_3 _returnvalue_4)))) 3e+02))
  (CallFunction|SetCenterPointAllAlive))

(event Custom|Set%20box%20position
  ;[1 1 1] for debugging
  (Transformation|SetWorldLocation (Variables|Default|GetBox) (Variables|Default|GetCenterPos) false false))

(event Custom|SetCenterPointAllAlive
  ;[1 1 1] set center point all alive
  (Variables|Default|SetCenterPos (/ (+ (Transformation|GetActorLocation (Game|GetPlayerCharacter 0)) (Transformation|GetActorLocation (Game|GetPlayerCharacter 1)) (Transformation|GetActorLocation (Game|GetPlayerCharacter 2)) (Transformation|GetActorLocation (Game|GetPlayerCharacter 3))) "4.000000,4.000000,4.000000")))

(event Custom|SetCamPos
  (bind _box (Variables|Default|GetBox))
  (bind _returnvalue (Transformation|GetWorldLocation _box))
  (bind (_x _y) (Math|Vector|BreakVector _returnvalue))
  (Variables|Default|SetCameraYpos (Math|Interpolation|FInterpTo (Variables|Default|GetCameraYpos) _y (Variables|Default|GetDelta) 3.0))
  (Variables|Default|SetCameraXpos (Math|Interpolation|FInterpTo (Variables|Default|GetCameraXpos) (- _x (Variables|Default|GetYoffSet)) (Variables|Default|GetDelta) 3.0))
  (Transformation|SetWorldLocation (Variables|Default|GetSpringArm) (Math|Vector|MakeVector (Variables|Default|GetCameraXpos) (Variables|Default|GetCameraYpos) (.Z (Math|Vector|BreakVector (Variables|Default|GetCameraStartPos)))) false false))

(event EventBeginPlay
  (bind _springarm (Variables|Default|GetSpringArm))
  (bind _returnvalue (Transformation|GetWorldLocation _springarm))
  (bind (_x _y) (Math|Vector|BreakVector _returnvalue))
  (Variables|Default|SetCameraXpos _x)
  (Variables|Default|SetCameraYpos _y)
  (Variables|Default|SetCameraStartPos (Math|Vector|MakeVector 0.0 0.0 (.Z (Math|Vector|BreakVector (Transformation|GetActorLocation))))))

(event EventTick
  (params (DeltaSeconds :type Float%20%28single-precision%29))
  (Variables|Default|SetDelta DeltaSeconds)
  (CallFunction|CameraZoom)
  (CallFunction|SetBoxPosition)
  (CallFunction|SetCamPos)
  (CallFunction|SetLongestPoint))

(fn ConstructionScript)