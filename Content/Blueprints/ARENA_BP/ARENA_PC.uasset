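; Arena Blueprint, apparently a player controller, that puts up to four local players into the characters chosen on the character selection screen.
; On BeginPlay it reads four selected character classes from gameinfoinstance, spawning each at the transform of player controllers 0 to 3 and possessing it.
; The players are handled in one sequential chain using global controller indices rather than self, with no check on player count.
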(event EventBeginPlay
  ;[1 1 1] control the character selected in the character selection screen
  (Utilities|FlowControl|Sequence
    (:then_0
      ;;[1 1 1] getting the character from the gameinfoinstance
      (bind _asgameinfoinstance (Utilities|Casting|CastTogameinfoinstance (Game|GetGameInstance)))
      ;;[1 1 1] setting and spawning the character selected
      (bind _output_get (Variables|/Game/Blueprints/gameinfoinstance.gameinfoinstance_C|Setselected%20character _asgameinfoinstance (Variables|/Game/Blueprints/gameinfoinstance.gameinfoinstance_C|Getselected%20character _asgameinfoinstance)))
      (bind _returnvalue (Game|SpawnActorfromClass _output_get (Transformation|GetActorTransform (Game|GetPlayerController 0)) "Undefined" 0 0))
      ;;[1 1 1] possesing the character
      (Pawn|Possess (Game|GetPlayerController 0) _returnvalue)
      ;[1 1 1] getting the character from the gameinfoinstance
      (bind _asgameinfoinstance_2 (Utilities|Casting|CastTogameinfoinstance (Game|GetGameInstance)))
      ;[1 1 1] setting and spawning the character selected
      (bind _output_get_2 (Variables|/Game/Blueprints/gameinfoinstance.gameinfoinstance_C|Setselected%20character_2 _asgameinfoinstance_2 (Variables|/Game/Blueprints/gameinfoinstance.gameinfoinstance_C|Getselected%20character_2 _asgameinfoinstance_2)))
      (bind _returnvalue_2 (Game|SpawnActorfromClass _output_get_2 (Transformation|GetActorTransform (Game|GetPlayerController 1)) "Undefined" 0 0))
      ;[1 1 1] possesing the character
      (Pawn|Possess (Game|GetPlayerController 1) _returnvalue_2)
      ;[1 1 1] getting the character from the gameinfoinstance
      (bind _asgameinfoinstance_3 (Utilities|Casting|CastTogameinfoinstance (Game|GetGameInstance)))
      ;[1 1 1] setting and spawning the character selected
      (bind _output_get_3 (Variables|/Game/Blueprints/gameinfoinstance.gameinfoinstance_C|Setselected%20character_3 _asgameinfoinstance_3 (Variables|/Game/Blueprints/gameinfoinstance.gameinfoinstance_C|Getselected%20character_3 _asgameinfoinstance_3)))
      (bind _returnvalue_3 (Game|SpawnActorfromClass _output_get_3 (Transformation|GetActorTransform (Game|GetPlayerController 2)) "Undefined" 0 0))
      ;[1 1 1] possesing the character
      (Pawn|Possess (Game|GetPlayerController 2) _returnvalue_3)
      ;[1 1 1] getting the character from the gameinfoinstance
      (bind _asgameinfoinstance_4 (Utilities|Casting|CastTogameinfoinstance (Game|GetGameInstance)))
      ;[1 1 1] setting and spawning the character selected
      (bind _output_get_4 (Variables|/Game/Blueprints/gameinfoinstance.gameinfoinstance_C|Setselected%20character_4 _asgameinfoinstance_4 (Variables|/Game/Blueprints/gameinfoinstance.gameinfoinstance_C|Getselected%20character_4 _asgameinfoinstance_4)))
      (bind _returnvalue_4 (Game|SpawnActorfromClass _output_get_4 (Transformation|GetActorTransform (Game|GetPlayerController 3)) "Undefined" 0 0))
      ;[1 1 1] possesing the character
      (Pawn|Possess (Game|GetPlayerController 3) _returnvalue_4))))

(event EventTick
  (params (DeltaSeconds :type Float%20%28single-precision%29)))

(fn ConstructionScript)