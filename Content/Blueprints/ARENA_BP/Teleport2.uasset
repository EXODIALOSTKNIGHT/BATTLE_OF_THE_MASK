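; Teleport2 is an arena Blueprint that plays a particle effect when the game instance flags it, apparently as teleport feedback.
; Tick polls the PlayParticle flag on gameinfoinstance and, after a short delay, activates the ParticleSystem component without reset.
; After a further two-second delay it clears the flag, so the shared game instance variable acts as the trigger.
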(event EventTick
  (params (DeltaSeconds :type Float%20%28single-precision%29))
  (bind _asgameinfoinstance (Utilities|Casting|CastTogameinfoinstance (Game|GetGameInstance)))
  (if (Variables|/Game/Blueprints/gameinfoinstance.gameinfoinstance_C|GetPlayParticle _asgameinfoinstance)
    (Utilities|FlowControl|Delay 0.1)
    (Components|Activation|Activate (Variables|Default|GetParticleSystem) false)
    (Utilities|FlowControl|Delay 2.0)
    (bind _asgameinfoinstance_2 (Utilities|Casting|CastTogameinfoinstance (Game|GetGameInstance)))
    (Variables|/Game/Blueprints/gameinfoinstance.gameinfoinstance_C|SetPlayParticle _asgameinfoinstance_2 false)))

(fn ConstructionScript)