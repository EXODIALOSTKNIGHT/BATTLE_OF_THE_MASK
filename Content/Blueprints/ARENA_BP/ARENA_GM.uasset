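; Arena game mode for a four-player local match that opens the WINNING_SCREEN level once at least three players are dead.
; BeginPlay creates the players, then spawns each character selected in gameinfoinstance at its controller's transform and possesses it.
; Tick polls the game instance's death flags, copies them locally and runs the win check.
; SpawnFunction looks up tagged PlayerStart transforms but is not called here.
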(event Custom|win%20condition
  ;[1 1 1] CHECK IF WHO IS THE WINNER
  (Utilities|FlowControl|Sequence
    (:then_0
      (if (Math|Boolean|ANDBoolean (Variables|Default|Getplayer%201%20dead) (Variables|Default|Getplayer%202%20dead) (Variables|Default|Getplayer%203%20dead))
        (Game|OpenLevel(byName) "WINNING_SCREEN" :!label _label)))
    (:then_1
      (if (Math|Boolean|ANDBoolean (Variables|Default|Getplayer%201%20dead) (Variables|Default|Getplayer%202%20dead) (Variables|Default|Getplayer%204%20dead))
        (goto _label)))
    (:then_2
      (if (Math|Boolean|ANDBoolean (Variables|Default|Getplayer%201%20dead) (Variables|Default|Getplayer%203%20dead) (Variables|Default|Getplayer%204%20dead))
        (goto _label)))
    (:then_3
      (if (Math|Boolean|ANDBoolean (Variables|Default|Getplayer%202%20dead) (Variables|Default|Getplayer%203%20dead) (Variables|Default|Getplayer%204%20dead))
        (goto _label)))
    (:then_4
      (if (Math|Boolean|ANDBoolean (Variables|Default|Getplayer%201%20dead) (Variables|Default|Getplayer%202%20dead) (Variables|Default|Getplayer%203%20dead) (Variables|Default|Getplayer%204%20dead))
        (goto _label)))))

(event EventTick
  (params (DeltaSeconds :type Float%20%28single-precision%29))
  ;[1 1 1] CHECKING IF THE PLAYER IS DEAD
  (Utilities|FlowControl|Sequence
    (:then_0
      ;;[1 1 1] GET THE INFORMATION FROM GAMEINSTANCE IF THE PLAYER IS DEAD
      (bind _asgameinfoinstance (Utilities|Casting|CastTogameinfoinstance (Game|GetGameInstance)))
      (if (Math|Boolean|Equal(Boolean) (Variables|/Game/Blueprints/gameinfoinstance.gameinfoinstance_C|Getplayer%201%20is%20dead _asgameinfoinstance) true)
        (Variables|Default|Setplayer%201%20dead true)
        (CallFunction|WinCondition)))
    (:then_1
      (bind _asgameinfoinstance_2 (Utilities|Casting|CastTogameinfoinstance (Game|GetGameInstance)))
      (if (Math|Boolean|Equal(Boolean) (Variables|/Game/Blueprints/gameinfoinstance.gameinfoinstance_C|Getplayer%202%20is%20dead _asgameinfoinstance_2) true)
        (Variables|Default|Setplayer%202%20dead true)
        (CallFunction|WinCondition)))
    (:then_2
      (bind _asgameinfoinstance_3 (Utilities|Casting|CastTogameinfoinstance (Game|GetGameInstance)))
      (if (Math|Boolean|Equal(Boolean) (Variables|/Game/Blueprints/gameinfoinstance.gameinfoinstance_C|Getplayer%203%20is%20dead _asgameinfoinstance_3) true)
        (Variables|Default|Setplayer%203%20dead true)
        (CallFunction|WinCondition)))
    (:then_3
      (bind _asgameinfoinstance_4 (Utilities|Casting|CastTogameinfoinstance (Game|GetGameInstance)))
      (if (Math|Boolean|Equal(Boolean) (Variables|/Game/Blueprints/gameinfoinstance.gameinfoinstance_C|Getplayer%204%20is%20dead _asgameinfoinstance_4) true)
        (Variables|Default|Setplayer%204%20dead true)
        (CallFunction|WinCondition)))))

(event EventBeginPlay
  (Class|GameplayStatics|CreatePlayer 0)
  (Class|GameplayStatics|CreatePlayer 1)
  (Class|GameplayStatics|CreatePlayer 2)
  (Class|GameplayStatics|CreatePlayer 3)
  ;[1 1 1] control the character selected in the character selection screen
  (Utilities|FlowControl|Sequence
    (:then_0
      ;;[1 1 1] getting the character from the gameinfoinstance
      (bind _asgameinfoinstance (Utilities|Casting|CastTogameinfoinstance (Game|GetGameInstance)))
      ;;[1 1 1] setting and spawning the character selected
      (bind _output_get (Variables|/Game/Blueprints/gameinfoinstance.gameinfoinstance_C|Setselected%20character _asgameinfoinstance (Variables|/Game/Blueprints/gameinfoinstance.gameinfoinstance_C|Getselected%20character _asgameinfoinstance)))
      (bind _returnvalue (Game|SpawnActorfromClass _output_get (Transformation|GetActorTransform (Game|GetPlayerController 0)) "Undefined" 0 0))
      ;;[1 1 1] possesing the character
      (Pawn|Possess (Game|GetPlayerController 0) _returnvalue))
    (:then_1
      ;[1 1 1] getting the character from the gameinfoinstance
      (bind _asgameinfoinstance_2 (Utilities|Casting|CastTogameinfoinstance (Game|GetGameInstance)))
      ;[1 1 1] setting and spawning the character selected
      (bind _output_get_2 (Variables|/Game/Blueprints/gameinfoinstance.gameinfoinstance_C|Setselected%20character_2 _asgameinfoinstance_2 (Variables|/Game/Blueprints/gameinfoinstance.gameinfoinstance_C|Getselected%20character_2 _asgameinfoinstance_2)))
      (bind _returnvalue_2 (Game|SpawnActorfromClass _output_get_2 (Transformation|GetActorTransform (Game|GetPlayerController 1)) "Undefined" 0 0))
      ;[1 1 1] possesing the character
      (Pawn|Possess (Game|GetPlayerController 1) _returnvalue_2))
    (:then_2
      ;[1 1 1] getting the character from the gameinfoinstance
      (bind _asgameinfoinstance_3 (Utilities|Casting|CastTogameinfoinstance (Game|GetGameInstance)))
      ;[1 1 1] setting and spawning the character selected
      (bind _output_get_3 (Variables|/Game/Blueprints/gameinfoinstance.gameinfoinstance_C|Setselected%20character_3 _asgameinfoinstance_3 (Variables|/Game/Blueprints/gameinfoinstance.gameinfoinstance_C|Getselected%20character_3 _asgameinfoinstance_3)))
      (bind _returnvalue_3 (Game|SpawnActorfromClass _output_get_3 (Transformation|GetActorTransform (Game|GetPlayerController 2)) "Undefined" 0 0))
      ;[1 1 1] possesing the character
      (Pawn|Possess (Game|GetPlayerController 2) _returnvalue_3))
    (:then_3
      ;[1 1 1] getting the character from the gameinfoinstance
      (bind _asgameinfoinstance_4 (Utilities|Casting|CastTogameinfoinstance (Game|GetGameInstance)))
      ;[1 1 1] setting and spawning the character selected
      (bind _output_get_4 (Variables|/Game/Blueprints/gameinfoinstance.gameinfoinstance_C|Setselected%20character_4 _asgameinfoinstance_4 (Variables|/Game/Blueprints/gameinfoinstance.gameinfoinstance_C|Getselected%20character_4 _asgameinfoinstance_4)))
      (bind _returnvalue_4 (Game|SpawnActorfromClass _output_get_4 (Transformation|GetActorTransform (Game|GetPlayerController 3)) "Undefined" 0 0))
      ;[1 1 1] possesing the character
      (Pawn|Possess (Game|GetPlayerController 3) _returnvalue_4))))

(fn ConstructionScript)

(fn SpawnFunction
  (bind _outactors (Actor|GetAllActorsOfClass "/Game/CHARACTERS/MASK_1/PlayerStart0.PlayerStart0_C"))
  (for _array_element _outactors
    (if (Utilities|Name|Equal(Name) (Variables|/Script/Engine.PlayerStart|GetPlayerStartTag _array_element) (Utilities|String|StringToName (Utilities|String|Append "player" (Utilities|String|ToString(Integer) (Variables|Default|GetPlayerInt)))))
      (Variables|Default|SetSpawnLocation (Transformation|GetActorTransform _array_element)))))