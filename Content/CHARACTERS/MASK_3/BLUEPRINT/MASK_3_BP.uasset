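; MASK_3 character Blueprint with movement input, a HUD and fireball damage.
; Four input axes push player character 0 along world X and Y, and BeginPlay adds the HUD3 widget to the viewport.
; Overlapping a fireball subtracts Health3 and spawns an explosion.
; While health is non-negative, it also destroys the fireball and switches the view to the arena camera stored in the game instance.
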(event EventBeginPlay
  ;[1 1 1] Show HUD3
  (bind _returnvalue (UserInterface|CreateWidget "/Game/UI/HUD3.HUD3_C"))
  (Variables|/Game/UI/HUD3.HUD3_C|SetHealth3_ProgressBar _returnvalue 0)
  (UserInterface|Viewport|AddtoViewport _returnvalue 0))

(event Collision|EventActorBeginOverlap
  (params (OtherActor :type Actor%20Object%20Reference))
  ;[1 1 1] on hit by fireball
  (bind _asfireball_bp (Utilities|Casting|CastTofireball_bp OtherActor))
  (bind _output_get (Variables|Default|SetHealth3 (- (Variables|Default|GetHealth3) 1e+01)))
  (Effects|SpawnEmitteratLocation "/Game/InfinityBladeEffects/Effects/FX_Monsters/FX_Monster_Gruntling/Bomber/P_FireBombExplosion.P_FireBombExplosion" (Transformation|GetActorLocation _asfireball_bp))
  (if (<= 0.0 _output_get)
    (Actor|DestroyActor _asfireball_bp)
    ;;[1 1 1] after the destroy actor, cast to gameinfoinstance will be executed and will get the reference of arena camera
    (bind _asgameinfoinstance (Utilities|Casting|CastTogameinfoinstance (Game|GetGameInstance)))
    (bind _output_get_2 (Variables|/Game/Blueprints/gameinfoinstance.gameinfoinstance_C|SetARENA_1_REF _asgameinfoinstance (Variables|/Game/Blueprints/gameinfoinstance.gameinfoinstance_C|GetARENA_1_REF _asgameinfoinstance)))
    (Game|Player|SetViewTargetwithBlend (Game|GetPlayerController 0) _output_get_2 0.0 "VTBlend_Linear" 0.0 false)))

(event Input|AxisEvents|InputAxisFORWARD
  (params (AxisValue :type Float%20%28single-precision%29))
  ;[1 1 1] Movements
  (Pawn|Input|AddMovementInput (Game|GetPlayerCharacter 0) (Math|Vector|MakeVector (* (Input|AxisValues|GetFORWARD) 1.0) 0.0 0.0) AxisValue false))

(event Input|AxisEvents|InputAxisBACKWARD
  (params (AxisValue :type Float%20%28single-precision%29))
  ;[1 1 1] Movements
  (Pawn|Input|AddMovementInput (Game|GetPlayerCharacter 0) (Math|Vector|MakeVector (* (Input|AxisValues|GetBACKWARD) -1.0) 0.0 0.0) AxisValue false))

(event Input|AxisEvents|InputAxisRIGHT
  (params (AxisValue :type Float%20%28single-precision%29))
  ;[1 1 1] Movements
  (Pawn|Input|AddMovementInput (Game|GetPlayerCharacter 0) (Math|Vector|MakeVector 0.0 (* (Input|AxisValues|GetRIGHT) 1.0) 0.0) AxisValue false))

(event Input|AxisEvents|InputAxisLEFT
  (params (AxisValue :type Float%20%28single-precision%29))
  ;[1 1 1] Movements
  (Pawn|Input|AddMovementInput (Game|GetPlayerCharacter 0) (Math|Vector|MakeVector 0.0 (* (Input|AxisValues|GetLEFT) -1.0) 0.0) AxisValue false))

(fn ConstructionScript)