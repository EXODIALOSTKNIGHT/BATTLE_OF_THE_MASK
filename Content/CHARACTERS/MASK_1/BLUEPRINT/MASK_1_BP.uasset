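; MASK_1_BP is a player character Blueprint with world-axis movement and a fireball skill.
; Four input axes each add movement input along a fixed world X or Y direction on player character 0.
; The First_Skill action halts and disables movement, spawns a Fireball_bp slightly above the character with its rotation, then restores walking after a short delay, using a Castingfireball flag to block recasting meanwhile.
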(event Input|ActionEvents|InputActionFirst_Skill
  (params (Key :type Key%20Structure))
  (bind _returnvalue (Transformation|GetActorTransform))
  (bind _charactermovement (Variables|Character|GetCharacterMovement))
  (bind (_location _rotation _scale) (Math|Transform|BreakTransform _returnvalue))
  (:Pressed
    (if (not (Variables|Default|Getcastingfireball))
      (Pawn|Components|CharacterMovement|DisableMovement _charactermovement)
      (Components|Movement|StopMovementImmediately _charactermovement)
      (Game|SpawnActorfromClass "/Game/CHARACTERS/MASK_1/BLUEPRINT/fireball_bp.fireball_bp_C" (Math|Transform|MakeTransform (+ _location "0, 0,50.000000") _rotation _scale) "Undefined" 0 0)
      (Variables|Default|Setcastingfireball true)
      (Utilities|FlowControl|Delay 0.2)
      (Variables|Default|Setcastingfireball false)
      (Pawn|Components|CharacterMovement|SetMovementMode (Variables|Character|GetCharacterMovement) "MOVE_Walking" 0))))

(event Input|AxisEvents|InputAxisFORWARD
  (params (AxisValue :type Float%20%28single-precision%29))
  ;[1 1 1] movements
  (Pawn|Input|AddMovementInput (Game|GetPlayerCharacter 0) (Math|Vector|MakeVector (* (Input|AxisValues|GetFORWARD) 1.0) 0.0 0.0) AxisValue false))

(event Input|AxisEvents|InputAxisBACKWARD
  (params (AxisValue :type Float%20%28single-precision%29))
  ;[1 1 1] movements
  (Pawn|Input|AddMovementInput (Game|GetPlayerCharacter 0) (Math|Vector|MakeVector (* (Input|AxisValues|GetBACKWARD) -1.0) 0.0 0.0) AxisValue false))

(event Input|AxisEvents|InputAxisRIGHT
  (params (AxisValue :type Float%20%28single-precision%29))
  ;[1 1 1] movements
  (Pawn|Input|AddMovementInput (Game|GetPlayerCharacter 0) (Math|Vector|MakeVector 0.0 (* (Input|AxisValues|GetRIGHT) 1.0) 0.0) AxisValue false))

(event Input|AxisEvents|InputAxisLEFT
  (params (AxisValue :type Float%20%28single-precision%29))
  ;[1 1 1] movements
  (Pawn|Input|AddMovementInput (Game|GetPlayerCharacter 0) (Math|Vector|MakeVector 0.0 (* (Input|AxisValues|GetLEFT) -1.0) 0.0) AxisValue false))

(fn ConstructionScript)