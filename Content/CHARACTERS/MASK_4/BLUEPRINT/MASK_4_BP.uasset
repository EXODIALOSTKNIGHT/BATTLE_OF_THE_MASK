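; MASK_4_BP is a playable fireball-casting character for an arena fight, moved along world X/Y axes and given a HUD4 widget on BeginPlay.
; Its first skill briefly halts movement to spawn a fireball, then refills a cooldown value through a delay loop.
; Overlapping snowball, water or metal balls explode, reduce health and are destroyed.
; At zero health the character destroys itself and player 0's view switches to the game instance's arena camera.
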(event EventBeginPlay
  ;[1 1 1] Show HUD4
  (bind _returnvalue (UserInterface|CreateWidget "/Game/UI/HUD4.HUD4_C" (Game|GetPlayerController 0)))
  (Variables|/Game/UI/HUD4.HUD4_C|SetHealth4_ProgressBar _returnvalue 0)
  (UserInterface|Viewport|AddtoViewport _returnvalue 0))

(event Collision|EventActorBeginOverlap
  (params (OtherActor :type Actor%20Object%20Reference))
  (Utilities|FlowControl|Sequence
    (:then_0
      ;[1 1 1] on hit by snowball
      (bind _assnowball_bp (Utilities|Casting|CastTosnowball_bp OtherActor))
      (Effects|SpawnEmitteratLocation "/Game/InfinityBladeEffects/Effects/FX_Monsters/FX_Monster_Gruntling/Bomber/P_FireBombExplosion.P_FireBombExplosion" (Transformation|GetActorLocation _assnowball_bp))
      (bind _output_get (Variables|Default|SetHealth (- (Variables|Default|GetHealth) 1e+01)))
      (if (<= _output_get 0.0)
        (Actor|DestroyActor _assnowball_bp)
        (Actor|DestroyActor)
        ;[1 1 1] after the destroy actor, cast to gameinfoinstance will be executed and will get the reference of arena camera
        (bind _asgameinfoinstance (Utilities|Casting|CastTogameinfoinstance (Game|GetGameInstance) :!label _label))
        (bind _output_get_2 (Variables|/Game/Blueprints/gameinfoinstance.gameinfoinstance_C|SetARENA_1_REF _asgameinfoinstance (Variables|/Game/Blueprints/gameinfoinstance.gameinfoinstance_C|GetARENA_1_REF _asgameinfoinstance)))
        (Game|Player|SetViewTargetwithBlend (Game|GetPlayerController 0) _output_get_2 0.0 "VTBlend_Linear" 0.0 false)
        (else
          (Actor|DestroyActor _assnowball_bp))))
    (:then_1
      ;[1 1 1] on hit by waterball
      (bind _aswater_ball (Utilities|Casting|CastTowater_ball OtherActor))
      (Effects|SpawnEmitteratLocation "/Game/InfinityBladeEffects/Effects/FX_Monsters/FX_Monster_Gruntling/Bomber/P_FireBombExplosion.P_FireBombExplosion" (Transformation|GetActorLocation _aswater_ball))
      (bind _output_get_3 (Variables|Default|SetHealth (- (Variables|Default|GetHealth) 1e+01)))
      (if (<= _output_get_3 0.0)
        (Actor|DestroyActor _aswater_ball)
        (Actor|DestroyActor)
        (goto _label)
        (else
          (Actor|DestroyActor _aswater_ball))))
    (:then_2
      ;[1 1 1] on hit by metalball
      (bind _asmetalball_bp (Utilities|Casting|CastTometalball_bp OtherActor))
      (Effects|SpawnEmitteratLocation "/Game/InfinityBladeEffects/Effects/FX_Monsters/FX_Monster_Gruntling/Bomber/P_FireBombExplosion.P_FireBombExplosion" (Transformation|GetActorLocation _asmetalball_bp))
      (bind _output_get_4 (Variables|Default|SetHealth (- (Variables|Default|GetHealth) 1e+01)))
      (if (<= _output_get_4 0.0)
        (Actor|DestroyActor _asmetalball_bp)
        (Actor|DestroyActor)
        (goto _label)
        (else
          (Actor|DestroyActor _asmetalball_bp))))))

(event Input|ActionEvents|InputActionFirst_Skill
  (params (Key :type Key%20Structure))
  (bind _returnvalue (Transformation|GetActorTransform))
  (bind _charactermovement (Variables|Character|GetCharacterMovement))
  (bind (_location _rotation _scale) (Math|Transform|BreakTransform _returnvalue))
  ;[1 1 1] First skill
  (:Pressed
    (if (>= (Variables|Default|GetFirst%20Skill%20Cool%20Down) 1.0)
      (if (not (Variables|Default|GetCasting%20Fire%20Ball))
        (Pawn|Components|CharacterMovement|DisableMovement _charactermovement)
        (Components|Movement|StopMovementImmediately _charactermovement)
        (Game|SpawnActorfromClass "/Game/CHARACTERS/MASK_4/BLUEPRINT/fireball_bp.fireball_bp_C" (Math|Transform|MakeTransform (+ _location "0, 0,50.000000") _rotation _scale) "Undefined" 0 0)
        (Variables|Default|SetCasting%20Fire%20Ball true)
        (Utilities|FlowControl|Delay 0.2)
        (Variables|Default|SetCasting%20Fire%20Ball false)
        (Pawn|Components|CharacterMovement|SetMovementMode (Variables|Character|GetCharacterMovement) "MOVE_Walking" 0)
        (Variables|Default|SetFirst%20Skill%20Cool%20Down 0.0)
        (if (> 1.0 (stale _output_get)) :!label _label
          (Variables|Default|SetFirst%20Skill%20Cool%20Down (+ (Variables|Default|GetFirst%20Skill%20Cool%20Down) 0.1))
          (Utilities|FlowControl|Delay 0.2)
          (goto _label))))))

(event Input|AxisEvents|InputAxisFORWARD
  (params (AxisValue :type Float%20%28single-precision%29))
  ;[1 1 1] Movements
  (Pawn|Input|AddMovementInput (Math|Vector|MakeVector (* (Input|AxisValues|GetFORWARD) 1.0) 0.0 0.0) AxisValue false))

(event Input|AxisEvents|InputAxisBACKWARD
  (params (AxisValue :type Float%20%28single-precision%29))
  ;[1 1 1] Movements
  (Pawn|Input|AddMovementInput (Math|Vector|MakeVector (* (Input|AxisValues|GetBACKWARD) -1.0) 0.0 0.0) AxisValue false))

(event Input|AxisEvents|InputAxisRIGHT
  (params (AxisValue :type Float%20%28single-precision%29))
  ;[1 1 1] Movements
  (Pawn|Input|AddMovementInput (Math|Vector|MakeVector 0.0 (* (Input|AxisValues|GetRIGHT) 1.0) 0.0) AxisValue false))

(event Input|AxisEvents|InputAxisLEFT
  (params (AxisValue :type Float%20%28single-precision%29))
  ;[1 1 1] Movements
  (Pawn|Input|AddMovementInput (Math|Vector|MakeVector 0.0 (* (Input|AxisValues|GetLEFT) -1.0) 0.0) AxisValue false))

(fn ConstructionScript)